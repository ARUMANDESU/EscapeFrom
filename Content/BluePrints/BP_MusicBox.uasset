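; BP_MusicBox is an actor that plays music from BP_Music actors placed on it and keeps a point count.
; When a BP_Music overlaps MusicDisk, its valid track plays as a 2D sound and its name fills MusicTitle.
; Ending that overlap stops the sound and clears the title.
; Separately, each end overlap on Box increments PointsNum and updates the Points text, with no filter on the actor.
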(event OnComponentBeginOverlap(MusicDisk)
  (params (OverlappedComponent :type Primitive%20Component%20Object%20Reference) (OtherActor :type Actor%20Object%20Reference) (OtherComp :type Primitive%20Component%20Object%20Reference) (OtherBodyIndex :type Integer) (bFromSweep :type Boolean) (SweepResult :type Hit%20Result%20Structure%20%28by%20ref%29))
  (bind _asbp_music (Utilities|Casting|CastToBP_Music OtherActor))
  (Utilities|IsValid (Variables|/Game/BluePrints/BP_Music.BP_Music_C|GetMusic _asbp_music)
    (:Is%20Valid
      (bind _returnvalue (Audio|SpawnSound2D (Variables|/Game/BluePrints/BP_Music.BP_Music_C|GetMusic _asbp_music) 1.0 1.0 0.0 0 false false))
      (Audio|Components|Audio|Play _returnvalue 0.0)
      (Rendering|Components|TextRender|SetText (Variables|Default|GetMusicTitle) (Variables|/Game/BluePrints/BP_Music.BP_Music_C|GetName _asbp_music)))))

(event OnComponentEndOverlap(MusicDisk)
  (params (OverlappedComponent :type Primitive%20Component%20Object%20Reference) (OtherActor :type Actor%20Object%20Reference) (OtherComp :type Primitive%20Component%20Object%20Reference) (OtherBodyIndex :type Integer))
  (Utilities|Casting|CastToBP_Music OtherActor)
  (Audio|Components|Audio|Stop (stale OnComponentBeginOverlap(MusicDisk) _returnvalue))
  (Rendering|Components|TextRender|SetText (Variables|Default|GetMusicTitle) (Class|KismetTextLibrary|GetEmptyText)))

(event OnComponentEndOverlap(Box)
  (params (OverlappedComponent :type Primitive%20Component%20Object%20Reference) (OtherActor :type Actor%20Object%20Reference) (OtherComp :type Primitive%20Component%20Object%20Reference) (OtherBodyIndex :type Integer))
  (bind _result (Math|Float|IncrementFloat (Variables|Default|GetPointsNum))
    (:%20%20
      (Rendering|Components|TextRender|SetText (Variables|Default|GetPoints) (Utilities|Text|ToText(Float) _result "HalfToEven")))))

(event EventBeginPlay)

(event Collision|EventActorBeginOverlap
  (params (OtherActor :type Actor%20Object%20Reference)))

(event EventTick
  (params (DeltaSeconds :type Float%20%28single-precision%29)))

(fn ConstructionScript)