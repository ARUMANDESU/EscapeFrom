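; Puzzle mini button actor that toggles a linked Platforms object between activated and deactivated.
; An overlap box enables input and opens a gate for BP_Character, letting Interact toggle the button, and a hit on the button mesh toggles it too.
; Press and Unpress both replay the same timeline to slide the button along local Y, then update the linked object's state and IsPressed flag.
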(event OnComponentBeginOverlap(Box)
  (params (OverlappedComponent :type Primitive%20Component%20Object%20Reference) (OtherActor :type Actor%20Object%20Reference) (OtherComp :type Primitive%20Component%20Object%20Reference) (OtherBodyIndex :type Integer) (bFromSweep :type Boolean) (SweepResult :type Hit%20Result%20Structure%20%28by%20ref%29))
  (bind _platforms (Variables|Default|GetPlatforms))
  (Input|EnableInput (Game|GetPlayerController 0))
  (Utilities|Casting|CastToBP_Character OtherActor)
  (Utilities|FlowControl|Gate true) ; enters at Open
)

(event OnComponentHit(Btn)
  (params (HitComponent :type Primitive%20Component%20Object%20Reference) (OtherActor :type Actor%20Object%20Reference) (OtherComp :type Primitive%20Component%20Object%20Reference) (NormalImpulse :type Vector :default "0, 0, 0") (Hit :type Hit%20Result%20Structure%20%28by%20ref%29))
  (bind _platforms (Variables|Default|GetPlatforms))
  (Utilities|IsValid _platforms
    (:Is%20Valid
      (if (Variables|/Game/PuzzleLogic/BP_Puzzle_Logic_Platform.BP_Puzzle_Logic_Platform_C|GetIsPressed? _platforms)
        (CallFunction|Unpress)
        (else
          (CallFunction|Press))))))

(event OnComponentEndOverlap(Box)
  (params (OverlappedComponent :type Primitive%20Component%20Object%20Reference) (OtherActor :type Actor%20Object%20Reference) (OtherComp :type Primitive%20Component%20Object%20Reference) (OtherBodyIndex :type Integer))
  (bind _platforms (Variables|Default|GetPlatforms))
  (Input|DisableInput (Game|GetPlayerController 0))
  (Utilities|Casting|CastToBP_Character OtherActor)
  (Utilities|FlowControl|Gate true) ; enters at Close
)

(event Custom|Press
  (bind _platforms (Variables|Default|GetPlatforms))
  (bind _btn (Variables|Default|GetBtn))
  (bind _relativelocation (Variables|/Script/Engine.SceneComponent|GetRelativeLocation _btn))
  (Utilities|FlowControl|Sequence
    (:then_0
      (bind _offset (Timeline|BtnPress PlayFromStart)
        (:Update
          (Transformation|SetRelativeLocation _btn (Math|Vector|MakeVector (.x _relativelocation) _offset (.z _relativelocation)) false false))))
    (:then_1
      (Default|Activated _platforms)
      (Variables|/Game/PuzzleLogic/BP_Puzzle_Logic_Platform.BP_Puzzle_Logic_Platform_C|SetIsPressed? _platforms true))))

(event Custom|Unpress
  (bind _platforms (Variables|Default|GetPlatforms))
  (bind _btn (Variables|Default|GetBtn))
  (bind _relativelocation (Variables|/Script/Engine.SceneComponent|GetRelativeLocation _btn))
  (Utilities|FlowControl|Sequence
    (:then_0
      (bind _offset (Timeline|BtnPress PlayFromStart)
        (:Update
          (Transformation|SetRelativeLocation _btn (Math|Vector|MakeVector (.x _relativelocation) _offset (.z _relativelocation)) false false))))
    (:then_1
      (Default|Deactivated _platforms)
      (Variables|/Game/PuzzleLogic/BP_Puzzle_Logic_Platform.BP_Puzzle_Logic_Platform_C|SetIsPressed? _platforms false))))

(event EventBeginPlay)

(event Collision|EventActorBeginOverlap
  (params (OtherActor :type Actor%20Object%20Reference)))

(event EventTick
  (params (DeltaSeconds :type Float%20%28single-precision%29)))

(event Input|ActionEvents|InputActionInteract
  (params (Key :type Key%20Structure :default "None"))
  (bind _platforms (Variables|Default|GetPlatforms))
  (:Pressed
    (Utilities|FlowControl|Gate true
      (:Exit
        (Utilities|IsValid _platforms
          (:Is%20Valid
            (if (Variables|/Game/PuzzleLogic/BP_Puzzle_Logic_Platform.BP_Puzzle_Logic_Platform_C|GetIsPressed? _platforms)
              (CallFunction|Unpress)
              (else
                (CallFunction|Press)))))))))

(fn ConstructionScript)