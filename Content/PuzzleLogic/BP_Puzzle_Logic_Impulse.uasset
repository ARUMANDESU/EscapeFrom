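; Puzzle logic actor that launches whatever begins overlapping its Box upward with a velocity-change impulse.
; Characters get their capsule temporarily switched to physics simulation, receive the character impulse, then have simulation turned off after a short delay.
; Anything else gets the separate object impulse on the overlapping component, applied at that actor's root location.
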(event OnComponentBeginOverlap(Box)
  (params (OverlappedComponent :type Primitive%20Component%20Object%20Reference) (OtherActor :type Actor%20Object%20Reference) (OtherComp :type Primitive%20Component%20Object%20Reference) (OtherBodyIndex :type Integer) (bFromSweep :type Boolean) (SweepResult :type Hit%20Result%20Structure%20%28by%20ref%29))
  (bind _rootcomponent (Variables|/Script/Engine.Actor|GetRootComponent OtherActor))
  (bind _returnvalue (Transformation|GetWorldLocation _rootcomponent))
  (bind _ascharacter (Utilities|Casting|CastToCharacter OtherActor)
    (:then
      (Physics|SetSimulatePhysics (Variables|/Script/Engine.Character|GetCapsuleComponent _ascharacter) true)
      (Utilities|FlowControl|Sequence
        (:then_0
          (Class|PrimitiveComponent|AddVelocityChangeImpulseatLocation (Variables|/Script/Engine.Character|GetCapsuleComponent _ascharacter) (Math|Vector|MakeVector 0.0 0.0 (Variables|Default|GetImpulseForCharacter)) _returnvalue "None"))
        (:then_1
          (Utilities|FlowControl|Delay 0.2)
          (Physics|SetSimulatePhysics (Variables|/Script/Engine.Character|GetCapsuleComponent _ascharacter) false))))
    (:CastFailed
      (Class|PrimitiveComponent|AddVelocityChangeImpulseatLocation OtherComp (Math|Vector|MakeVector 0.0 0.0 (Variables|Default|GetImpulseForObjects)) _returnvalue "None"))))

(event EventBeginPlay)

(event Collision|EventActorBeginOverlap
  (params (OtherActor :type Actor%20Object%20Reference)))

(event EventTick
  (params (DeltaSeconds :type Float%20%28single-precision%29)))

(fn ConstructionScript)