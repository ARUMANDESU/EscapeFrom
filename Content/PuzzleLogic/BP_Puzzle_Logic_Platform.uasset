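; BP_Puzzle_Logic_Platform is a puzzle-logic moving platform that travels along a spline when activated and returns when deactivated.
; Activated sets the MovePlatform timeline's play rate from TimeToMove and plays it, while Deactivated reverses it.
; Each timeline update lerps the distance along the Road spline and moves the Platform component to that world location without sweeping.
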(event Collision|EventActorBeginOverlap
  (params (OtherActor :type Actor%20Object%20Reference)))

(event EventBeginPlay)

(event EventActivated
  (Components|Timeline|SetPlayRate (Variables|Default|GetMovePlatform) (/ 1.0 (Variables|Default|GetTimeToMove)))
  (bind _movetrack (Timeline|MovePlatform Play)
    (:Update
      (Transformation|SetWorldLocation (Variables|Default|GetPlatform) (Spline|GetLocationatDistanceAlongSpline (Variables|Default|GetRoad) (Math|Float|Lerp 0.0 (Spline|GetSplineLength (Variables|Default|GetRoad)) _movetrack) "World") false false))))

(event EventDeactivated
  (bind _movetrack (Timeline|MovePlatform Reverse)
    (:Update
      (Transformation|SetWorldLocation (Variables|Default|GetPlatform) (Spline|GetLocationatDistanceAlongSpline (Variables|Default|GetRoad) (Math|Float|Lerp 0.0 (Spline|GetSplineLength (Variables|Default|GetRoad)) _movetrack) "World") false false))))

(fn ConstructionScript)