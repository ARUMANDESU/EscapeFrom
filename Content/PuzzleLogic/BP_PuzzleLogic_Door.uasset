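; BP_PuzzleLogic_Door is a puzzle door that opens once a required number of buttons are active.
; Activated and Deactivated events raise and lower a counter that is compared against the Buttons total.
; Reaching the total plays the Door timeline, which moves two door cubes on Z through separate Bottom and Upper tracks.
; Dropping below the total reverses the timeline.
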(event EventBeginPlay)

(event Collision|EventActorBeginOverlap
  (params (OtherActor :type Actor%20Object%20Reference)))

(event EventDeactivated
  (bind _result (Math|Integer|DecrementInt (Variables|Default|GetBtnTimes))
    (:%20%20
      (if (< _result (Variables|Default|GetButtons))
        (bind (_direction _upper _bottom) (Timeline|Door Reverse)
          (:Update
            (Transformation|SetRelativeLocation (Variables|Default|GetEscapeDoor_Cube) (Math|Vector|MakeVector 0.0 0.0 _bottom) false false)
            (Transformation|SetRelativeLocation (Variables|Default|GetEscapeDoor_Cube_001) (Math|Vector|MakeVector 0.0 0.0 _upper) false false)))))))

(event EventTick
  (params (DeltaSeconds :type Float%20%28single-precision%29)))

(event EventActivated
  (bind _result (Math|Integer|IncrementInt (Variables|Default|GetBtnTimes))
    (:%20%20
      (if (== _result (Variables|Default|GetButtons))
        (bind (_direction _upper _bottom) (Timeline|Door Play)
          (:Update
            (Transformation|SetRelativeLocation (Variables|Default|GetEscapeDoor_Cube) (Math|Vector|MakeVector 0.0 0.0 _bottom) false false)
            (Transformation|SetRelativeLocation (Variables|Default|GetEscapeDoor_Cube_001) (Math|Vector|MakeVector 0.0 0.0 _upper) false false)))))))

(fn ConstructionScript)