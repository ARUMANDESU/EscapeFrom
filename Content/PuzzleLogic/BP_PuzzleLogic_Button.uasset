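; Puzzle pressure button that activates or deactivates an array of doors when a matching object overlaps it.
; Overlapping components qualify only if their first material equals the button's Material or the ForAllBtn material, so materials act as keys.
; A timeline lowers or raises ShapeCube1 along Z and reverses on end overlap, which also flips the doors' state.
; IsPrevending inverts the logic, deactivating doors on press and activating them on release.
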(event OnComponentBeginOverlap(btn)
  (params (OverlappedComponent :type Primitive%20Component%20Object%20Reference) (OtherActor :type Actor%20Object%20Reference) (OtherComp :type Primitive%20Component%20Object%20Reference) (OtherBodyIndex :type Integer) (bFromSweep :type Boolean) (SweepResult :type Hit%20Result%20Structure%20%28by%20ref%29))
  (bind _returnvalue (Rendering|Material|GetMaterial OtherComp 0))
  (bind _door (Variables|Default|GetDoor))
  (if (or (== _returnvalue (Variables|Default|GetMaterial)) (== _returnvalue (Variables|Default|GetForAllBtn)))
    (Utilities|FlowControl|Sequence
      (:then_0
        (bind _offset (Timeline|Timeline_0 Play)
          (:Update
            (Transformation|SetRelativeLocation (Variables|Default|GetShape_Cube1) (Math|Vector|MakeVector 0.0 0.0 _offset) false false))))
      (:then_1
        (if (Variables|Default|GetIsPrevending)
          (for _array_element _door
            (Default|Deactivated _array_element))
          (else
            (for _array_element_2 _door
              (Default|Activated _array_element_2))))))))

(event OnComponentEndOverlap(btn)
  (params (OverlappedComponent :type Primitive%20Component%20Object%20Reference) (OtherActor :type Actor%20Object%20Reference) (OtherComp :type Primitive%20Component%20Object%20Reference) (OtherBodyIndex :type Integer))
  (bind _returnvalue (Rendering|Material|GetMaterial OtherComp 0))
  (bind _door (Variables|Default|GetDoor))
  (if (or (== _returnvalue (Variables|Default|GetMaterial)) (== _returnvalue (Variables|Default|GetForAllBtn)))
    (Utilities|FlowControl|Sequence
      (:then_0
        (bind _offset (Timeline|Timeline_0 Reverse)
          (:Update
            (Transformation|SetRelativeLocation (Variables|Default|GetShape_Cube1) (Math|Vector|MakeVector 0.0 0.0 _offset) false false))))
      (:then_1
        (if (Variables|Default|GetIsPrevending)
          (for _array_element _door
            (Default|Activated _array_element))
          (else
            (for _array_element_2 _door
              (Default|Deactivated _array_element_2))))))))

(event EventBeginPlay
  (Rendering|Material|SetMaterial (Variables|Default|GetShape_Cube1) 0 (Variables|Default|GetMaterial)))

(event Collision|EventActorBeginOverlap
  (params (OtherActor :type Actor%20Object%20Reference)))

(event EventTick
  (params (DeltaSeconds :type Float%20%28single-precision%29)))

(fn ConstructionScript)